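; BP_WaterGoal is a goal trigger that completes the level when the player pawn's move count equals its maximum.
; Its TriggerAction event reads both counts from BP_PlayerPawn and does nothing unless they match.
; On a match, it sets the pawn's TickTimer flag and shows UI_Modal_LevelComplete with the pawn's elapsed seconds.
; BeginPlay and the construction script only call the parent class.
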(event EventBeginPlay
  (|CallParentFunction))

(event EventTriggerAction
  (bind _asbp_player_pawn (Utilities|Casting|CastToBP_PlayerPawn (Game|Player|GetPlayerPawn 0)))
  (if (== (Variables|/Game/Hydrogen/Blueprints/Player/BP_PlayerPawn.BP_PlayerPawn_C|GetMoveCount _asbp_player_pawn) (Variables|/Game/Hydrogen/Blueprints/Player/BP_PlayerPawn.BP_PlayerPawn_C|GetMaxMoveCount _asbp_player_pawn))
    (bind _asbp_player_pawn_2 (Utilities|Casting|CastToBP_PlayerPawn (Game|Player|GetPlayerPawn 0)))
    (Variables|/Game/Hydrogen/Blueprints/Player/BP_PlayerPawn.BP_PlayerPawn_C|SetTickTimer _asbp_player_pawn_2 true)
    (bind _returnvalue (UserInterface|CreateWidget "/Game/Hydrogen/Widgets/UI_Modal_LevelComplete.UI_Modal_LevelComplete_C"))
    (Variables|/Game/Hydrogen/Widgets/UI_Modal_LevelComplete.UI_Modal_LevelComplete_C|SetCurrentSeconds _returnvalue (Variables|/Game/Hydrogen/Blueprints/Player/BP_PlayerPawn.BP_PlayerPawn_C|GetCurrentSeconds _asbp_player_pawn_2))
    (UserInterface|Viewport|AddtoViewport _returnvalue 66)))

(fn ConstructionScript
  (|CallParentFunction))