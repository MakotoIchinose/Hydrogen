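; Player pawn that relays directional input to a mover and reports elapsed time and move counts to the HUD.
; On BeginPlay it possesses itself, sets game-only input without a cursor, caches the BP_WidgetSecretary HUD and starts its play display.
; Move presses go to MoverRef as interface messages while IsControlling is set.
; Tick accumulates time for the HUD while TickTimer is set, and UpdateMove pushes current and maximum move counts.
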(event EventBeginPlay)

(event Collision|EventActorBeginOverlap
  (params (OtherActor :type Actor%20Object%20Reference)))

(event EventTick
  (params (DeltaSeconds :type Float%20%28single-precision%29)))

(event Custom|UpdateMove
  (Default|UpdateMoves (Variables|Default|GetHUDRef) (Variables|Default|GetMoveCount) (Variables|Default|GetMaxMoveCount)))

(event EventBeginPlay
  (bind _returnvalue (Game|GetPlayerController 0))
  (Pawn|Possess _returnvalue self)
  (Input|SetInputModeGameOnly _returnvalue false)
  (Variables|/Script/Engine.PlayerController|SetbShowMouseCursor _returnvalue false)
  (bind _asbp_widget_secretary (Utilities|Casting|CastToBP_WidgetSecretary (HUD|GetHUD _returnvalue)))
  (bind _output_get (Variables|Default|SetHUDRef _asbp_widget_secretary))
  (Default|StartPlay _output_get)
  (CallFunction|UpdateMove))

(event EventTick
  (params (DeltaSeconds :type Float%20%28single-precision%29))
  (if (Variables|Default|GetTickTimer)
    (bind _output_get (Variables|Default|SetCurrentSeconds (+ DeltaSeconds (Variables|Default|GetCurrentSeconds))))
    (Default|UpdateTimer (Variables|Default|GetHUDRef) _output_get)))

(event Input|ActionEvents|InputActionMoveUp
  (params (Key :type Key%20Structure :default "None"))
  (:Pressed
    (if (Variables|Default|GetIsControlling)
      (Class|BPIControls|MoveUpInterface(Message) (Variables|Default|GetMoverRef)))))

(event Input|ActionEvents|InputActionMoveDown
  (params (Key :type Key%20Structure :default "None"))
  (:Pressed
    (if (Variables|Default|GetIsControlling)
      (Class|BPIControls|MoveDownInterface(Message) (Variables|Default|GetMoverRef)))))

(event Input|ActionEvents|InputActionMoveLeft
  (params (Key :type Key%20Structure :default "None"))
  (:Pressed
    (if (Variables|Default|GetIsControlling)
      (Class|BPIControls|MoveLeftInterface(Message) (Variables|Default|GetMoverRef)))))

(event Input|ActionEvents|InputActionMoveRight
  (params (Key :type Key%20Structure :default "None"))
  (:Pressed
    (if (Variables|Default|GetIsControlling)
      (Class|BPIControls|MoveRightInterface(Message) (Variables|Default|GetMoverRef)))))

(fn ConstructionScript)