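; Planteid root trunk segment actor whose SetMaterial function gives its Sphere a dynamic M_Planteid_RootTrunk material instance.
; As wired, it ignores both direction inputs and always applies one fixed Index.
; An unconnected branch tree holds unused tile selection: random variants for straight runs, fixed indices for corners, from last and current direction.
; The event graph and construction script are empty.
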(event EventBeginPlay)

(event Collision|EventActorBeginOverlap
  (params (OtherActor :type Actor%20Object%20Reference)))

(event EventTick
  (params (DeltaSeconds :type Float%20%28single-precision%29)))

(fn ConstructionScript)

(fn SetMaterial
  (params (LastDirection :type Vector) (CurrentDirection :type Vector))
  (bind _returnvalue (Rendering|Material|CreateDynamicMaterialInstance "/Game/Hydrogen/Material/Planteid/M_Planteid_RootTrunk.M_Planteid_RootTrunk" "None" "None" :!class /Script/Engine.KismetMaterialLibrary))
  (Rendering|Material|SetScalarParameterValue _returnvalue "Index" 8.0 :!class /Script/Engine.MaterialInstanceDynamic)
  (Rendering|Material|SetMaterial (Variables|Default|GetSphere) 0 _returnvalue))