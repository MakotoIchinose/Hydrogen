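; Planteid core actor that anchors a grid-grown root system and spawns a BP_Planteid_Mover linked back to it on BeginPlay.
; CollisionCheck traces for roots, obstacles or cores, and CreateStep spawns root segments, tracking the last root and offset.
; SetMaterial picks the core's directional material by Index on a dynamic instance.
; The input interface events are empty, their old step-and-retexture logic is disconnected, and RootMaterialBend is an unfinished stub.
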(event EventBeginPlay
  (bind _returnvalue (Game|SpawnActorfromClass "/Game/Hydrogen/Blueprints/Planteid/BP_Planteid_Mover.BP_Planteid_Mover_C" (Transformation|GetActorTransform) "Undefined" 0 0))
  (Variables|/Game/Hydrogen/Blueprints/Planteid/BP_Planteid_Mover.BP_Planteid_Mover_C|SetCoreActor _returnvalue self))

(event EventMoveRightInterface)

(event EventMoveLeftInterface)

(event EventMoveDownInterface)

(event EventMoveUpInterface)

(fn ConstructionScript)

(fn CollisionCheck
  (params (Target :type Vector))
  (bind _returnvalue (Transformation|GetActorLocation))
  (bind _lasttransform (Variables|Default|GetLastTransform))
  (bind _lastroot (Variables|Default|GetLastRoot))
  (bind _returnvalue_2 (+ _returnvalue _lasttransform))
  (bind _outhit (Collision|LineTraceByChannel _returnvalue_2 (+ _returnvalue_2 Target) "TraceTypeQuery1" false (Utilities|Array|MakeArray (select (Utilities|IsValid _lastroot) _lastroot self)) "ForDuration" false))
  (return (Math|Boolean|ORBoolean (== (Utilities|GetClass (.HitActor (Collision|BreakHitResult _outhit))) "/Game/Hydrogen/Blueprints/Planteid/BP_Planteid_Root.BP_Planteid_Root_C") (== (Utilities|GetClass (.HitActor (Collision|BreakHitResult _outhit))) "/Game/Hydrogen/Blueprints/Obstacle/BP_Obstacle.BP_Obstacle_C") (== (Utilities|GetClass (.HitActor (Collision|BreakHitResult _outhit))) "BP_PlanteidCore_C"))))

(fn CreateStep
  (params (Offset :type Vector))
  (bind _returnvalue (Game|SpawnActorfromClass "/Game/Hydrogen/Blueprints/Planteid/BP_Planteid_Root.BP_Planteid_Root_C" (Math|Transform|MakeTransform (+ (+ (Variables|Default|GetLastTransform) Offset) (Transformation|GetActorLocation)) "0, 0, 0" "1.000000,1.000000,1.000000") "Undefined" 0 0))
  (Variables|Default|SetLastRoot _returnvalue)
  (Variables|Default|SetLastTransform (+ (Variables|Default|GetLastTransform) Offset)))

(fn RootMaterialBend
  (params (PreviousDirection :type Vector) (CurrentDirection :type Vector))
  (Utilities|FlowControl|Sequence
    (:then_0
      (Utilities|FlowControl|Sequence
        (:then_0
          (if (or (and (Utilities|Operators|EqualEqual PreviousDirection "0.000000,-1.000000,0.000000" 0.0) (Utilities|Operators|EqualEqual CurrentDirection "-1.000000,0.000000,0.000000" 0.0)) (and (Utilities|Operators|EqualEqual PreviousDirection "1.000000,0.000000,0.000000" 0.0) (Utilities|Operators|EqualEqual CurrentDirection "0.000000,1.000000,0.000000" 0.0)))
            _))
        (:then_1
          (if (or (and (Utilities|Operators|EqualEqual PreviousDirection "0.000000,-1.000000,0.000000" 0.0) (Utilities|Operators|EqualEqual CurrentDirection "-1.000000,0.000000,0.000000" 0.0)) (and (Utilities|Operators|EqualEqual PreviousDirection "1.000000,0.000000,0.000000" 0.0) (Utilities|Operators|EqualEqual CurrentDirection "0.000000,1.000000,0.000000" 0.0)))
            _))
        (:then_2
          (if (or (and (Utilities|Operators|EqualEqual PreviousDirection "0.000000,-1.000000,0.000000" 0.0) (Utilities|Operators|EqualEqual CurrentDirection "-1.000000,0.000000,0.000000" 0.0)) (and (Utilities|Operators|EqualEqual PreviousDirection "1.000000,0.000000,0.000000" 0.0) (Utilities|Operators|EqualEqual CurrentDirection "0.000000,1.000000,0.000000" 0.0)))
            _))
        (:then_3
          (if (or (and (Utilities|Operators|EqualEqual PreviousDirection "0.000000,-1.000000,0.000000" 0.0) (Utilities|Operators|EqualEqual CurrentDirection "-1.000000,0.000000,0.000000" 0.0)) (and (Utilities|Operators|EqualEqual PreviousDirection "1.000000,0.000000,0.000000" 0.0) (Utilities|Operators|EqualEqual CurrentDirection "0.000000,1.000000,0.000000" 0.0)))
            _))))
    (:then_1
      (Rendering|Material|CreateDynamicMaterialInstance 0 "None" "None" :!class /Script/Engine.KismetMaterialLibrary))))

(fn SetMaterial
  (params (Direction :type Vector))
  (bind _returnvalue (Math|Float|MakeLiteralFloat 1.0))
  (Rendering|Material|CreateDynamicMaterialInstance 0 "None" "None" :!class /Script/Engine.KismetMaterialLibrary)
  (if (Utilities|Operators|EqualEqual Direction "0.000000,100.000000,0.000000" _returnvalue)
    (bind _returnvalue_2 (Rendering|Material|CreateDynamicMaterialInstance "/Game/Hydrogen/Material/Planteid/M_Planteid_Core.M_Planteid_Core" "None" "None" :!class /Script/Engine.KismetMaterialLibrary))
    (Rendering|Material|SetScalarParameterValue _returnvalue_2 "Index" 1.0 :!class /Script/Engine.MaterialInstanceDynamic)
    (Rendering|Material|SetMaterial (Variables|Default|GetSphere) 0 _returnvalue_2)
    (elif (Utilities|Operators|EqualEqual Direction "0.000000,-100.000000,0.000000" _returnvalue)
      (bind _returnvalue_3 (Rendering|Material|CreateDynamicMaterialInstance "/Game/Hydrogen/Material/Planteid/M_Planteid_Core.M_Planteid_Core" "None" "None" :!class /Script/Engine.KismetMaterialLibrary))
      (Rendering|Material|SetScalarParameterValue _returnvalue_3 "Index" 3.0 :!class /Script/Engine.MaterialInstanceDynamic)
      (Rendering|Material|SetMaterial (Variables|Default|GetSphere) 0 _returnvalue_3)
      (elif (Utilities|Operators|EqualEqual Direction "-100.000000,0.000000,0.000000" _returnvalue)
        (bind _returnvalue_4 (Rendering|Material|CreateDynamicMaterialInstance "/Game/Hydrogen/Material/Planteid/M_Planteid_Core.M_Planteid_Core" "None" "None" :!class /Script/Engine.KismetMaterialLibrary))
        (Rendering|Material|SetScalarParameterValue _returnvalue_4 "Index" 2.0 :!class /Script/Engine.MaterialInstanceDynamic)
        (Rendering|Material|SetMaterial (Variables|Default|GetSphere) 0 _returnvalue_4)
        (elif (Utilities|Operators|EqualEqual Direction "100.000000,0.000000,0.000000" _returnvalue)
          (bind _returnvalue_5 (Rendering|Material|CreateDynamicMaterialInstance "/Game/Hydrogen/Material/Planteid/M_Planteid_Core.M_Planteid_Core" "None" "None" :!class /Script/Engine.KismetMaterialLibrary))
          (Rendering|Material|SetScalarParameterValue _returnvalue_5 "Index" 4.0 :!class /Script/Engine.MaterialInstanceDynamic)
          (Rendering|Material|SetMaterial (Variables|Default|GetSphere) 0 _returnvalue_5))))))