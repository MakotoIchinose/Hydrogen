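; Grid-stepping tip of the Planteid that grows a trail of roots from its core as the player moves it, registering itself with BP_PlayerPawn.
; Interface move events call CreateStep, which line-traces to block steps into core, roots or obstacles.
; A valid step spawns a root behind (except the first), swaps direction-indexed trunk materials on tip and previous piece, and updates the pawn's move count.
; A short trace then fires any BP_Trigger hit.
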(event EventMoveRightInterface
  (CallFunction|CreateStep "0.000000,100.000000,0.000000"))

(event EventMoveLeftInterface
  (CallFunction|CreateStep "0.000000,-100.000000,0.000000"))

(event EventMoveDownInterface
  (CallFunction|CreateStep "-100.000000,0.000000,0.000000"))

(event EventMoveUpInterface
  (CallFunction|CreateStep "100.000000,0.000000,0.000000"))

(event EventBeginPlay
  (bind _returnvalue (Actor|GetActorOfClass "/Game/Hydrogen/Blueprints/Player/BP_PlayerPawn.BP_PlayerPawn_C"))
  (Variables|/Game/Hydrogen/Blueprints/Player/BP_PlayerPawn.BP_PlayerPawn_C|SetMoverRef _returnvalue self))

(fn ConstructionScript)

(fn CollisionCheck
  (params (Target :type Vector))
  (bind _returnvalue (Transformation|GetActorLocation))
  (bind _outhit (Collision|LineTraceByChannel _returnvalue (+ _returnvalue Target) "TraceTypeQuery1" false (Utilities|Array|MakeArray (select (Utilities|IsValid (Variables|Default|GetLastRoot)) 0 (Variables|Default|GetCoreActor))) "None"))
  (if (Math|Boolean|ORBoolean (Utilities|ClassIsChildOf (Utilities|GetClass (.HitActor (Collision|BreakHitResult _outhit))) "/Game/Hydrogen/Blueprints/Planteid/BP_PlanteidCore.BP_PlanteidCore_C") (Utilities|ClassIsChildOf (Utilities|GetClass (.HitActor (Collision|BreakHitResult _outhit))) "/Game/Hydrogen/Blueprints/Planteid/BP_Planteid_Root.BP_Planteid_Root_C") (Utilities|ClassIsChildOf (Utilities|GetClass (.HitActor (Collision|BreakHitResult _outhit))) "/Game/Hydrogen/Blueprints/Obstacle/BP_Obstacle.BP_Obstacle_C"))
    (return true)
    (else
      (return false))))

(fn CreateStep
  (params (Offset :type Vector))
  (bind _isblocked (CallFunction|CollisionCheck Offset))
  (if (not _isblocked)
    (Development|PrintString (Utilities|String|ToString(Vector) Offset) true true "(R=1.000000,G=0.082384,B=0.000000,A=1.000000)")
    (Development|PrintString (Utilities|String|ToString(Vector) (Variables|Default|GetLastPosition)) true true "(R=0.305177,G=1.000000,B=0.000000,A=1.000000)")
    (bind _asbp_player_pawn (Utilities|Casting|CastToBP_PlayerPawn (Game|Player|GetPlayerPawn 0)))
    (if (== (Variables|/Game/Hydrogen/Blueprints/Player/BP_PlayerPawn.BP_PlayerPawn_C|GetMoveCount _asbp_player_pawn) 0)
      (Development|SetHiddeninGame (Variables|Default|GetSphere) false false)
      (Transformation|AddActorLocalOffset Offset false true)
      (else
        (bind _returnvalue (Game|SpawnActorfromClass "/Game/Hydrogen/Blueprints/Planteid/BP_Planteid_Root.BP_Planteid_Root_C" (Math|Transform|MakeTransform (Transformation|GetActorLocation) "0, 0, 0" "1.000000,1.000000,1.000000") "Undefined" 0 0))
        (Variables|Default|SetLastRoot _returnvalue)
        (Transformation|AddActorLocalOffset Offset false true)))
    (CallFunction|SetMaterial Offset)
    (Utilities|IsValid (Variables|Default|GetLastRoot)
      (:Is%20Valid
        (Default|SetMaterial (Variables|Default|GetLastRoot) (Variables|Default|GetLastDirection) Offset))
      (:Is%20Not%20Valid
        (Default|SetMaterial (Variables|Default|GetCoreActor) Offset)))
    (Variables|Default|SetLastDirection Offset)
    (bind _asbp_player_pawn_2 (Utilities|Casting|CastToBP_PlayerPawn (Game|Player|GetPlayerPawn 0)))
    (Math|Integer|IncrementInt (Variables|/Game/Hydrogen/Blueprints/Player/BP_PlayerPawn.BP_PlayerPawn_C|GetMoveCount _asbp_player_pawn_2)
      (:%20%20
        (Default|UpdateMove _asbp_player_pawn_2)
        (CallFunction|CheckTrigger)))))

(fn NewFunction)

(fn UpdatePointer
  (Transformation|SetWorldLocation (Variables|Default|GetWidget) (+ (Variables|Default|GetLastPosition) (Transformation|GetActorLocation)) false true))

(fn SetMaterial
  (params (Direction :type Vector))
  (if (Utilities|Operators|EqualEqual Direction "0.000000,100.000000,0.000000" 1.0)
    (bind _returnvalue (Rendering|Material|CreateDynamicMaterialInstance "/Game/Hydrogen/Material/Planteid/M_Planteid_RootTrunk.M_Planteid_RootTrunk" "None" "None" :!class /Script/Engine.KismetMaterialLibrary))
    (Rendering|Material|SetScalarParameterValue _returnvalue "Index" 5.0 :!class /Script/Engine.MaterialInstanceDynamic)
    (Rendering|Material|SetMaterial (Variables|Default|GetSphere) 0 _returnvalue)
    (elif (Utilities|Operators|EqualEqual Direction "0.000000,-100.000000,0.000000" 1.0)
      (bind _returnvalue_2 (Rendering|Material|CreateDynamicMaterialInstance "/Game/Hydrogen/Material/Planteid/M_Planteid_RootTrunk.M_Planteid_RootTrunk" "None" "None" :!class /Script/Engine.KismetMaterialLibrary))
      (Rendering|Material|SetScalarParameterValue _returnvalue_2 "Index" 5.0 :!class /Script/Engine.MaterialInstanceDynamic)
      (Rendering|Material|SetMaterial (Variables|Default|GetSphere) 0 _returnvalue_2)
      (elif (Utilities|Operators|EqualEqual Direction "-100.000000,0.000000,0.000000" 1.0)
        (bind _returnvalue_3 (Rendering|Material|CreateDynamicMaterialInstance "/Game/Hydrogen/Material/Planteid/M_Planteid_RootTrunk.M_Planteid_RootTrunk" "None" "None" :!class /Script/Engine.KismetMaterialLibrary))
        (Rendering|Material|SetScalarParameterValue _returnvalue_3 "Index" 6.0 :!class /Script/Engine.MaterialInstanceDynamic)
        (Rendering|Material|SetMaterial (Variables|Default|GetSphere) 0 _returnvalue_3)
        (elif (Utilities|Operators|EqualEqual Direction "100.000000,0.000000,0.000000" 1.0)
          (bind _returnvalue_4 (Rendering|Material|CreateDynamicMaterialInstance "/Game/Hydrogen/Material/Planteid/M_Planteid_RootTrunk.M_Planteid_RootTrunk" "None" "None" :!class /Script/Engine.KismetMaterialLibrary))
          (Rendering|Material|SetScalarParameterValue _returnvalue_4 "Index" 13.0 :!class /Script/Engine.MaterialInstanceDynamic)
          (Rendering|Material|SetMaterial (Variables|Default|GetSphere) 0 _returnvalue_4))))))

(fn CheckTrigger
  (bind _returnvalue (Transformation|GetActorLocation))
  (bind _outhit (Collision|LineTraceByChannel _returnvalue (+ _returnvalue "0.000000,1.000000,0.000000") "TraceTypeQuery1" false 0 "ForDuration"))
  (Development|PrintString (Utilities|GetDisplayName (.HitActor (Collision|BreakHitResult _outhit))))
  (bind _asbp_trigger (Utilities|Casting|CastToBP_Trigger (.HitActor (Collision|BreakHitResult _outhit))))
  (Class|BPITriggers|TriggerAction(Message) _asbp_trigger))